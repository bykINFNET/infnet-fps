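; BP_Weapon is a weapon actor that the player can collect and that tracks its own ammo.
; On interact, it checks the interacting actor for the Player tag and sends that actor a collect-weapon interface message with itself.
; AddAmmo raises extra ammo up to its maximum and prints the total, while CheckMaxAmmo reports whether current ammo is below its limit.
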(event `/Game/MyProject/BluePrints/Interfaces/BPI_Interaction.I_Interact`
  (params (I_Actor :type "Actor Object Reference"))
  (if (`self.ActorHasTag` I_Actor "Player")
    (message `/Game/MyProject/BluePrints/Interfaces/BPI_Interaction.I_CollectWeapon` I_Actor self)))

(event `Event AddAmmo`
  (params (numAmmo :type Integer))
  (bind _output_get (set `self.currentExtraAmmo` (`KismetMathLibrary.Min` (+ numAmmo (`self.currentExtraAmmo`)) (`self.maxExtraAmmo`))))
  (`KismetSystemLibrary.PrintString` (`KismetStringLibrary.Conv_IntToString` _output_get)))

(fn `checkMaxAmmo`
  (returns (canAddAmmo :type Boolean))
  (return (< (`self.currentAmmo`) (`self.maxAmmo`))))

(fn `UserConstructionScript`)